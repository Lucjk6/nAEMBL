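; Actor Blueprint that moves its Cube component along a circular path around the actor's origin.
; Each Tick adds Speed to an angle accumulator, Sum, and uses cosine and sine in degrees scaled by Raggio to set the cube's relative X and Y at a fixed height.
; The step is not scaled by delta time, so the orbit speed depends on frame rate.
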(event `self.ReceiveBeginPlay`)

(event `self.ReceiveTick`
  (params (DeltaSeconds :type "Float (single-precision)"))
  (bind _raggio (`self.Raggio`))
  (bind _output_get (set `self.Sum` (+ (`self.Sum`) (`self.Speed`))))
  (`SceneComponent.K2_SetRelativeLocation` (`self.Cube`) (`KismetMathLibrary.MakeVector` (* (`KismetMathLibrary.DegCos` _output_get) _raggio) (* _raggio (`KismetMathLibrary.DegSin` _output_get)) 145.0) false false))

(fn `UserConstructionScript`)